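; HealOrb is a pickup that adds a fixed amount of health to the player character.
; BeginPlay caches the player as BP_ThirdPersonCharacter.
; When that player overlaps SphereColl, it hides the orb and sphere and increases Health in the character's BPCStats component, without a clamp.
; The actor is neither destroyed nor has its collision disabled, so re-entering the hidden sphere heals again.
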(event `self.ReceiveBeginPlay`
  (bind _asbp_third_person_character (cast `/Game/ThirdPerson/Blueprints/BP_ThirdPersonCharacter` (`GameplayStatics.GetPlayerCharacter` 0)))
  (set `self.As BP Third Person Character` _asbp_third_person_character))

(event `self.SphereColl.OnComponentBeginOverlap`
  (params (OverlappedComponent :type "PrimitiveComponent Object Reference") (OtherActor :type "Actor Object Reference") (OtherComp :type "PrimitiveComponent Object Reference") (OtherBodyIndex :type Integer) (bFromSweep :type Boolean) (SweepResult :type "HitResult Structure (by ref)"))
  (bind _bpc_stats (`/Game/ThirdPerson/Blueprints/BP_ThirdPersonCharacter.BPC_Stats` (`self.As BP Third Person Character`)))
  (if (== (`GameplayStatics.GetPlayerCharacter` 0) OtherActor)
    (`SceneComponent.SetVisibility` (`self.greenorb`) false false)
    (`SceneComponent.SetVisibility` (`self.SphereColl`) false false)
    (set `/Game/ThirdPerson/Stats/BPC_Stats.Health` (+ (`/Game/ThirdPerson/Stats/BPC_Stats.Health` _bpc_stats) 5.0) _bpc_stats)))

(fn `UserConstructionScript`)