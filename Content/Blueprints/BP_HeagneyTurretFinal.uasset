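; BP_HeagneyTurretFinal is a turret that rotates and fires on a timer, though its logic is disconnected from BeginPlay and never runs.
; The TurretMovement timeline yaws Base toward RotationAmt, restarting for full 360-degree turns and otherwise ping-ponging.
; A parallel Delay loop spawns a plain Actor at Arrow and sets ProjectileMovement's max speed.
; TurretAnimSpeed scales both timeline rate and fire interval, so faster turning means faster firing.
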(event `self.ReceiveBeginPlay`)

(fn `UserConstructionScript`)