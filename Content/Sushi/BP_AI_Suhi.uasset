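; AI controller for the Sushi AI that runs a behavior tree and drives it through blackboard keys.
; PawnSensing sightings flag the seen pawn as the target, yet write the same state value as SetStateAsPassive.
; Helper functions switch the E_AI_States key between passive, attack with a target, and investigate with a location.
; Patrol route, movement speed and the shadow and punch attack functions are empty stubs.
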(event `self.ReceiveBeginPlay`
  (`self.RunBehaviorTree` (`self.BehaviorTree`)))

(event `self.PawnSensing.OnSeePawn`
  (params (Pawn :type "Pawn Object Reference"))
  (`BlackboardComponent.SetValueAsBool` (`AIBlueprintHelperLibrary.GetBlackboard` null) "SeeingTarget?" true)
  (`BlackboardComponent.SetValueAsObject` (`AIBlueprintHelperLibrary.GetBlackboard` null) "TargetActor" Pawn)
  (set `self.Attack_target` Pawn)
  (`BlackboardComponent.SetValueAsEnum` (`AIBlueprintHelperLibrary.GetBlackboard` null) (`self.State Key Name`) (enumliteral `/Game/AI/Enums/E_AI_States` "NewEnumerator0")))

(fn `GetPatrolRoute`
  (returns (PatrolRoute :type "/Game/AI/AI_Patrol_Route Object Reference"))
  (return null))

(fn `SetMovementSpeed`
  (params (Speed :type "/Game/AI/Enums/E_MovementSpeed Enum" :default "NewEnumerator0"))
  (returns (SpeedValue :type "Float (double-precision)"))
  (return 0.0))

(fn `SetStateAsAttack`
  (params (`Attack Target` :type "Actor Object Reference"))
  (`BlackboardComponent.SetValueAsObject` (`AIBlueprintHelperLibrary.GetBlackboard` null) "TargetActor" `Attack Target`)
  (`BlackboardComponent.SetValueAsEnum` (`AIBlueprintHelperLibrary.GetBlackboard` null) (`self.State Key Name`) (enumliteral `/Game/AI/Enums/E_AI_States` "NewEnumerator1")))

(fn `SetStateAsInvestigate`
  (params (Location :type "Vector Structure"))
  (`BlackboardComponent.SetValueAsEnum` (`AIBlueprintHelperLibrary.GetBlackboard` null) (`self.State Key Name`) (enumliteral `/Game/AI/Enums/E_AI_States` "NewEnumerator3"))
  (`BlackboardComponent.SetValueAsVector` (`AIBlueprintHelperLibrary.GetBlackboard` null) (`self.PointOfInterestKeyName`) Location))

(fn `SetStateAsPassive`
  (`BlackboardComponent.SetValueAsEnum` (`AIBlueprintHelperLibrary.GetBlackboard` null) (`self.State Key Name`) (enumliteral `/Game/AI/Enums/E_AI_States` "NewEnumerator0")))

(fn `ShadowGrab`
  (returns (Duration :type "Float (double-precision)"))
  (return 0.0))

(fn `ShadowKick_grab_FUP`
  (returns (Duration :type "Float (double-precision)"))
  (return 0.0))

(fn `UserConstructionScript`)

(fn `WeakPunchAttack`
  (returns (Duration :type "Float (double-precision)"))
  (return 0.0))