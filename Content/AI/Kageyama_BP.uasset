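; Kageyama enemy character with montage attacks (weak punch, shadow kick, shadow grab), a proximity-revealed health bar and a lock-on widget.
; A looping timer runs sphere traces that apply throttled damage and flag player hits during the grab's one-second window.
; A successful grab attaches the player, then detaches and launches them.
; Incoming damage feeds BPCStats, while Die ragdolls the mesh, hides the health bar and stops trace damage.
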(event `self.DisplayLockedOnWidget`
  (params (ShowWidget :type Boolean))
  (`SceneComponent.SetVisibility` (`self.LockOnWidget`) ShowWidget false))

(event `self.ReceiveBeginPlay`
  (bind _asenemy_healthbar_widget (cast `/Game/AI/Enemy_Healthbar_Widget` (`WidgetComponent.GetWidget` (`self.Enemy_HealthWidget`))))
  (`/Game/ThirdPerson/Stats/BPC_Stats.Set Health Progress Bar` (`self.BPC_Stats`) (`/Game/AI/Enemy_Healthbar_Widget.EnemyHealth` _asenemy_healthbar_widget)))

(event `self.ReceiveAnyDamage`
  (params (Damage :type "Float (single-precision)") (DamageType :type "DamageType Object Reference") (InstigatedBy :type "Controller Object Reference") (DamageCauser :type "Actor Object Reference"))
  (`/Game/ThirdPerson/Stats/BPC_Stats.Increase Value` (`self.BPC_Stats`) "NewEnumerator0" (* Damage -1.0)))

(event `self.End Attack Trace`
  ;[1 1 1] Attack Traces
  (if (`KismetSystemLibrary.K2_IsValidTimerHandle` (stale `self.Begin Attack Trace` _returnvalue))
    (`KismetSystemLibrary.K2_ClearAndInvalidateTimerHandle` (stale `self.Begin Attack Trace` _returnvalue))))

(event `self.Begin Attack Trace`
  ;[1 1 1] Attack Traces
  (bind _returnvalue (`KismetSystemLibrary.K2_SetTimerDelegate` (delegate `DamageTrace`) 0.08 true)))

(event `DamageTrace`
  (bind _returnvalue (`SceneComponent.K2_GetComponentLocation` (`self.Sphere`)))
  ;[1 1 1] Attack Traces
  (if (not (`self.IsDead`))
    (bind (_outhit _returnvalue_2) (`KismetSystemLibrary.SphereTraceSingleForObjects` :`Start` _returnvalue :`End` (+ _returnvalue (50.0 0.0 0.0)) :`Radius` 50.0 :`ObjectTypes` (`|MakeArray` "ObjectTypeQuery3" :!type "EObjectTypeQuery Enum") :`DrawDebugType` "ForDuration" :`DrawTime` 2.0))
    (bind (_bblockinghit _binitialoverlap _time _distance _location _impactpoint _normal _impactnormal _physmat _hitactor) (`GameplayStatics.BreakHitResult` _outhit))
    (set `self.HitActor` _hitactor)
    (if _returnvalue_2
      (if (and (`self.CheckGrabStart`) (== (`self.HitActor`) (`GameplayStatics.GetPlayerCharacter` 0)))
        (set `self.CheckGrabEnd` true)
        (else
          (set `self.CheckGrabEnd` false)))
      (`/Engine/EditorBlueprintResources/StandardMacros.DoOnce` false :!label _label
        (:`Completed`
          (`GameplayStatics.ApplyDamage` _hitactor (`self.AttackDamage`))
          (`KismetSystemLibrary.Delay` 0.3)
          (goto _label :!via `Reset`))))))

(event `self.ReceiveHit`
  (params (MyComp :type "PrimitiveComponent Object Reference") (Other :type "Actor Object Reference") (OtherComp :type "PrimitiveComponent Object Reference") (bSelfMoved :type Boolean) (HitLocation :type "Vector Structure") (HitNormal :type "Vector Structure") (NormalImpulse :type "Vector Structure") (Hit :type "HitResult Structure (by ref)")))

(event `self.Die`
  (`CharacterMovementComponent.DisableMovement` (`self.CharacterMovement`))
  (`PrimitiveComponent.SetSimulatePhysics` (`self.Mesh`) true)
  (set `self.IsDead` true)
  (`SceneComponent.SetVisibility` (`self.Enemy_HealthWidget`) false false)
  (`ActorComponent.K2_DestroyComponent` (`self.SphereColl`)))

(event `self.DetectHealthBar.OnComponentBeginOverlap`
  (params (OverlappedComponent :type "PrimitiveComponent Object Reference") (OtherActor :type "Actor Object Reference") (OtherComp :type "PrimitiveComponent Object Reference") (OtherBodyIndex :type Integer) (bFromSweep :type Boolean) (SweepResult :type "HitResult Structure (by ref)"))
  (bind _asbp_third_person_character (cast `/Game/ThirdPerson/Blueprints/BP_ThirdPersonCharacter` (`GameplayStatics.GetPlayerCharacter` 0)))
  (if (== _asbp_third_person_character OtherActor)
    (if (not (`self.IsDead`))
      (`SceneComponent.SetVisibility` (`self.Enemy_HealthWidget`) true false))))

(event `ShadowG_Start`
  (bind _returnvalue (`GameplayStatics.GetPlayerCharacter` 0))
  (bind _returnvalue_2 (`GameplayStatics.GetPlayerCharacter` 0))
  (set `self.CheckGrabStart` true)
  (`KismetSystemLibrary.Delay` 1.0)
  (set `self.CheckGrabStart` false)
  (if (`self.CheckGrabEnd`)
    (`self.K2_AttachToActor` _returnvalue self "None" "SnapToTarget" "KeepRelative" "KeepRelative" true)
    (`CharacterMovementComponent.SetMovementMode` (`Character.CharacterMovement` _returnvalue) "MOVE_None" 0)
    (`KismetSystemLibrary.Delay` 1.3)
    (`self.K2_DetachFromActor` _returnvalue_2 "KeepWorld" "KeepWorld" "KeepWorld")
    (`CharacterMovementComponent.SetMovementMode` (`Character.CharacterMovement` _returnvalue_2) "MOVE_Walking" 0)
    (`self.LaunchCharacter` _returnvalue_2 (* (+ (`self.GetActorForwardVector`) (0.0 10.0 1.5)) 1000.0) true true)
    (`KismetSystemLibrary.Delay` 3.0)
    (`KismetSystemLibrary.PrintString` "throw complete")))

(fn `ShadowGrab`
  (returns (Duration :type "Float (double-precision)"))
  (bind _returnvalue (`self.PlayAnimMontage` "/Game/RetargetedAnims/All_Retargeted/NormalAttacks_RT/ShadowGrab_Montage.ShadowGrab_Montage"))
  (`self.ShadowG_Start`)
  (return _returnvalue))

(fn `ShadowKick_grab_FUP`
  (returns (Duration :type "Float (double-precision)"))
  (bind _returnvalue (`self.PlayAnimMontage` "/Game/RetargetedAnims/All_Retargeted/Combos/Combo3/ShadowKick_Montage.ShadowKick_Montage"))
  (return _returnvalue))

(fn `UserConstructionScript`)

(fn `WeakPunchAttack`
  (returns (Duration :type "Float (double-precision)"))
  (bind _returnvalue (`self.PlayAnimMontage` "/Game/RetargetedAnims/All_Retargeted/Combos/Combo5/BasicEnemyBnb.BasicEnemyBnb"))
  (return _returnvalue))