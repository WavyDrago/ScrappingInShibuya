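; AI controller for the Kageyama boss that reveals the boss health bar when it first spots the player.
; PawnSensing sightings pass through a DoOnce, which resets if the seen pawn is not BP_ThirdPersonCharacter.
; On a player sighting, it adds the controlled Kageyama_BP's health bar widget to the top vertical box of the player's HUD.
; SetStateAsAttack only calls the parent implementation.
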(event `self.PawnSensing.OnSeePawn`
  (params (Pawn :type "Pawn Object Reference"))
  (`/Engine/EditorBlueprintResources/StandardMacros.DoOnce` false :!label _label
    (:`Completed`
      (bind _asbp_third_person_character (cast `/Game/ThirdPerson/Blueprints/BP_ThirdPersonCharacter` Pawn)
        (:`then`
          (bind _askageyama_bp (cast `/Game/AI/Kageyama_BP` (`self.K2_GetPawn`)))
          (`VerticalBox.AddChildToVerticalBox` (`/Game/MyMainMenu/Combat_UI/Hud_health_Widget.Top_VerticalBox` (`/Game/ThirdPerson/Blueprints/BP_ThirdPersonCharacter.HudRef` _asbp_third_person_character)) (`/Game/AI/Kageyama_BP.BossHealthBar_Widget` _askageyama_bp)))
        (:`CastFailed`
          (goto _label :!via `Reset`))))))

(fn `SetStateAsAttack`
  (params (`Attack Target` :type "Actor Object Reference"))
  (`parent.SetStateAsAttack` `Attack Target`))

(fn `UserConstructionScript`
  (`parent.UserConstructionScript`))