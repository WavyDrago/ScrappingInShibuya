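; FollowUPDragon_BP is a skill cinematic actor that lays out a segmented body, apparently for a dragon, from instanced static meshes.
; The construction script rebuilds the ISM from BodyCount, placing uniformly scaled-down boxlike segments at even spacing along negative X.
; No follow motion runs: LerpBoxs is an empty event, and the code that caches and updates instance transforms is disconnected.
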(event `LerpBoxs`)

(fn `UserConstructionScript`
  (`InstancedStaticMeshComponent.ClearInstances` (`self.ISM`))
  (for _index (range (+ (`self.BodyCount`) 1))
    (`InstancedStaticMeshComponent.AddInstance` (`self.ISM`) (`KismetMathLibrary.MakeTransform` (`KismetMathLibrary.MakeVector` (`KismetMathLibrary.Conv_IntToDouble` (* _index -50))) (struct) (0.4 0.3 0.5)) false)))